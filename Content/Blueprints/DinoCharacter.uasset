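; Player dino character that runs forward automatically along its control yaw, starting after a short delay from BeginPlay, and jumps on input.
; Jumping drives three parallel timelines for gravity scale, capsule half-height and mesh Z offset to shape the arc and collision.
; Releasing Jump plays a separate fall-gravity timeline, and landing restores normal gravity.
; Jump and landing set the State enum on ABP_Dino, which also blocks repeated jumps.
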(event `self.ReceiveBeginPlay`
  (`WidgetBlueprintLibrary.SetFocusToGameViewport`)
  (`KismetSystemLibrary.Delay` 3.0)
  (set `self.IsStarted` true))

(event `self.ReceiveTick`
  (params (DeltaSeconds :type "Float (single-precision)"))
  (if (`self.IsStarted`)
    (`self.AddMovementInput` (`KismetMathLibrary.GetForwardVector` (`KismetMathLibrary.MakeRotator` 0.0 0.0 (.yaw (`self.GetControlRotation`)))) (`self.Speed`))))

(event `InputAction|Jump`
  (params (Key :type "Key Structure"))
  (:`Pressed`
    (if (`self.IsStarted`)
      (bind _asabp_dino (cast `/Game/Blueprints/ABP_Dino` (`SkeletalMeshComponent.GetAnimInstance` (`self.Mesh`))))
      (if (`|EnumInequality` (`/Game/Blueprints/ABP_Dino.State` _asabp_dino) "NewEnumerator3")
        (`self.SetAnimState` "NewEnumerator3")
        (`self.Jump`)
        (`|ExecutionSequence`
          (:`then_0`
            (bind (_direction _gravity) (`Timeline|JumpGravityTimeline` :!via `PlayFromStart`)
              (:`Update`
                (set `CharacterMovementComponent.GravityScale` _gravity (`self.CharacterMovement`)))))
          (:`then_1`
            (bind (_direction_2 _capsulehalfheight) (`Timeline|JumpCapsuleHalfHeightTimeline` :!via `PlayFromStart`)
              (:`Update`
                (`CapsuleComponent.SetCapsuleHalfHeight` (`self.CapsuleComponent`) _capsulehalfheight true))))
          (:`then_2`
            (bind (_direction_3 _locationz) (`Timeline|JumpMeshLocationZTimeline` :!via `PlayFromStart`)
              (:`Update`
                (`SceneComponent.K2_SetRelativeLocation` (`self.Mesh`) (`KismetMathLibrary.MakeVector` 0.0 0.0 _locationz) false false))))))))
  (:`Released`
    (bind (_direction_4 _gravity_2) (`Timeline|FallGravityTimeline` :!via `PlayFromStart`)
      (:`Update`
        (set `CharacterMovementComponent.GravityScale` _gravity_2 (`self.CharacterMovement`))))))

(event `self.OnLanded`
  (params (Hit :type "HitResult Structure (by ref)"))
  (if (`self.IsStarted`)
    (`self.SetAnimState` "NewEnumerator1")
    (set `CharacterMovementComponent.GravityScale` 1.0 (`self.CharacterMovement`))))

(fn `SetAnimState`
  (params (State :type "/Game/Blueprints/DinoState Enum" :default "NewEnumerator0"))
  (bind _asabp_dino (cast `/Game/Blueprints/ABP_Dino` (`SkeletalMeshComponent.GetAnimInstance` (`self.Mesh`))))
  (set `/Game/Blueprints/ABP_Dino.State` State _asabp_dino))

(fn `UserConstructionScript`)